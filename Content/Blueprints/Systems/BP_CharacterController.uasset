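; Player controller that sets up the local player's UI and toggles a high-ping warning.
; On BeginPlay, local controllers create and store pause menu and HUD widgets, but only the HUD is added to the viewport.
; It then binds to show and hide Wi-Fi delegates, with warning events that toggle the HUD's high-ping image.
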(event `self.ReceiveBeginPlay`
  (if (`self.IsLocalPlayerController`)
    (bind _returnvalue (`|CreateWidget` "/Game/Widgets/WBP_PauseMenu.WBP_PauseMenu_C" self))
    (set `self.PauseMenuRef` _returnvalue)
    (bind _returnvalue_2 (`|CreateWidget` "/Game/Widgets/WBP_Hud.WBP_Hud_C" self))
    (bind _output_get (set `self.Hud_Ref` _returnvalue_2))
    (`/Engine/EditorBlueprintResources/StandardMacros.IsValid` _output_get
      (:`Is Valid`
        (`UserWidget.AddToViewport` _output_get 0)
        (add `self.M_ShowWifi` (`|CreateDelegate` :!event `ShowWifiWarning`))
        (add `self.M_HideWifi` (`|CreateDelegate` :!event `HideWifiWarning`))))))

(event `ShowWifiWarning`
  (`Widget.SetVisibility` (`/Game/Widgets/WBP_Hud.HighPingImage` (`self.Hud_Ref`)) "Visible"))

(event `HideWifiWarning`
  (`Widget.SetVisibility` (`/Game/Widgets/WBP_Hud.HighPingImage` (`self.Hud_Ref`)) "Hidden"))

(fn `UserConstructionScript`)