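; MenuPlayerController sets up the game's front-end menu interface on BeginPlay.
; It finds the DataHolderActor, uses its FirstController reference to create, show and activate the main menu widget, then enables the cursor and UI-only input.
; It also pre-creates the Play, Create Server, Join Server and Find Servers widgets and stores their references without adding them to the viewport.
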(event `self.ReceiveBeginPlay`
  (bind _first_controller (`self.GetFirstPlayerController`))
  (bind _returnvalue (`GameplayStatics.GetActorOfClass` "/Script/CoopProject.DataHolderActor"))
  (set `self.DataHolderRef` _returnvalue)
  (bind _firstcontroller (`DataHolderActor.FirstController` _returnvalue))
  (bind _returnvalue_2 (`|CreateWidget` "/Game/Widgets/WBP_MainMenu_UI.WBP_MainMenu_UI_C" _firstcontroller))
  (bind _output_get (set `self.MenuRef` _returnvalue_2))
  (`UserWidget.AddToViewport` _returnvalue_2 0)
  (`UserWidget.AddToViewport` _output_get 0)
  (`CommonActivatableWidget.ActivateWidget` _returnvalue_2)
  (set `PlayerController.bShowMouseCursor` true _firstcontroller)
  (`WidgetBlueprintLibrary.SetInputMode_UIOnlyEx` _firstcontroller null)
  (bind _returnvalue_3 (`|CreateWidget` "/Game/Widgets/WBP_CreateServer.WBP_CreateServer_C" _first_controller))
  (set `self.CreateServerRef` _returnvalue_3)
  (bind _returnvalue_4 (`|CreateWidget` "/Game/Widgets/WBP_JoinServer.WBP_JoinServer_C" _first_controller))
  (set `self.JoinSessionRef` _returnvalue_4)
  (bind _returnvalue_5 (`|CreateWidget` "/Game/Widgets/WBP_PlayMenu.WBP_PlayMenu_C" _first_controller))
  (set `self.PlayMenu` _returnvalue_5)
  (bind _returnvalue_6 (`|CreateWidget` "/Game/Widgets/WBP_FindServers.WBP_FindServers_C" _first_controller))
  (set `self.FindServersMenu` _returnvalue_6))

(fn `UserConstructionScript`)