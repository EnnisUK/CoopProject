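; BP_TriggerActor is an actor that switches how its mesh replicates physics, with debug output.
; On BeginPlay it binds SwitchPhysics to the MSwitchPhysics event dispatcher.
; When fired, the handler sets the mesh's ReplicatePhysicsToAutonomousProxy flag to whether the passed OwnerActor has authority, printing that actor's name and the result.
; The construction script and OnRep_NewVar are empty.
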(event `self.ReceiveBeginPlay`
  (add `self.M_SwitchPhysics` (delegate `SwitchPhysics`)))

(event `SwitchPhysics` :!signature `self.M_SwitchPhysics`
  (params (OwnerActor :type "Actor Object Reference"))
  (bind _m_mesh (`self.M_Mesh`))
  (`KismetSystemLibrary.PrintString` (`KismetSystemLibrary.GetDisplayName` OwnerActor))
  (if (`self.HasAuthority` OwnerActor)
    (bind _output_get (set `PrimitiveComponent.bReplicatePhysicsToAutonomousProxy` true _m_mesh))
    (`KismetSystemLibrary.PrintString` (`KismetStringLibrary.Conv_BoolToString` _output_get))
    (else
      (bind _output_get_2 (set `PrimitiveComponent.bReplicatePhysicsToAutonomousProxy` false _m_mesh))
      (`KismetSystemLibrary.PrintString` (`KismetStringLibrary.Conv_BoolToString` _output_get_2)))))

(fn `OnRep_NewVar`)

(fn `UserConstructionScript`)